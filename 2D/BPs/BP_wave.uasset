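; BP_wave is an enemy wave spawner that releases a set number of BP_Enemy actors when its SpawnEnemy event is called.
; It loops through a Delay, spawning one enemy per second at a fixed X with a random Y offset and decrementing NumOfEnemy.
; Each enemy receives fixed HP and speed through SetEnemyData, and a debug message prints once the count runs out.
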(event `SpawnEnemy`
  (if (> (`self.NumOfEnemy`) 0) :!label _label
    (bind _returnvalue (`|SpawnActorFromClass` "/Game/BPs/BP_Enemy.BP_Enemy_C" (`KismetMathLibrary.MakeTransform` (`KismetMathLibrary.MakeVector` 1000.0 (- (* (`KismetMathLibrary.RandomFloat`) 600.0) 300.0))) "Undefined" "OverrideRootScale" null null))
    (`/Game/BPs/BP_Enemy.SetEnemyData` _returnvalue 60.0 2.0)
    (set `self.NumOfEnemy` (- (`self.NumOfEnemy`) 1))
    (`KismetSystemLibrary.Delay` 1.0)
    (goto _label)
    (else
      (`KismetSystemLibrary.PrintString` "spawned all!"))))

(fn `UserConstructionScript`)