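; BP_Enemy is a wave enemy that walks a fixed serpentine path and takes projectile damage.
; Tick picks its movement offset from hardcoded world X/Y thresholds, scaled by the speed passed to SetEnemyData.
; It shows HP on a text render and tracks bullets targeting it.
; At zero HP it spawns an explosion, destroys remaining tracked bullets, removes itself from the Wave's array and destroys itself.
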(event `self.ReceiveTick`
  (params (DeltaSeconds :type "Float (single-precision)"))
  (bind _x (.x (`self.Enemylocation`)))
  (bind _y (.y (`self.Enemylocation`)))
  (`|ExecutionSequence`
    (:`then_0`
      (set `self.Enemylocation` (`self.K2_GetActorLocation`))
      (`self.K2_AddActorLocalOffset` (`self.MoveTo`)))
    (:`then_1`
      ;[1 1 1] 적 이동
      (if (and (> _x 9100.0) (>= _y 10900.0))
        (set `self.MoveTo` (`KismetMathLibrary.MakeVector` (* (`self.movespeed`) -4.0)) :!label _label)
        (elif (>= _y 10450.0)
          (set `self.MoveTo` (`KismetMathLibrary.MakeVector` 0.0 (* (`self.movespeed`) -4.0)) :!label _label_2)
          (else
            (if (and (< _x 11000.0) (>= _y 10300.0))
              _
              (elif (>= _y 10000.0)
                (goto _label_2)
                (elif (and (> _x 9100.0) (>= _y 9900.0))
                  (goto _label)
                  (elif (>= _y 9550.0)
                    (goto _label_2)
                    (elif (and (< _x 11000.0) (>= _y 9450.0))
                      _
                      (elif (>= _y 9100.0)
                        (goto _label_2)
                        (else
                          (goto _label))))))))
            (set `self.MoveTo` (`KismetMathLibrary.MakeVector` (* (`self.movespeed`) 4.0)))))))))

(event `SetEnemyData`
  (params (hp :type "Float (double-precision)") (speed :type "Float (double-precision)"))
  ;[1 1 1] 적 스탯 세팅
  (set `self.hp` hp)
  (set `self.movespeed` speed)
  (`self.Refresh Text`))

(event `targetedBybullet`
  (params (bullet :type "/Game/BPs/BP_Bullet Object Reference"))
  ;[1 1 1] 적을 향해 날아오는 투사체들 저장
  (`KismetArrayLibrary.Array_Add` (`self.TargetedBybullets`) bullet))

(event `GetAttacked`
  (params (damage :type "Float (double-precision)") (bulletDamaged :type "/Game/BPs/BP_Bullet Object Reference"))
  (bind _hp (`self.hp`))
  ;[1 1 1] 적 데미지 계산
  (`KismetArrayLibrary.Array_RemoveItem` (`self.TargetedBybullets`) bulletDamaged)
  (if (> _hp 0.0)
    (set `self.hp` (- _hp damage))
    (if (> (`self.hp`) 0.0)
      (`self.Refresh Text`)
      (else
        (set `self.hp` 0.0)))
    (`KismetSystemLibrary.PrintString` (`KismetStringLibrary.Conv_DoubleToString` _hp) false)
    (if (<= (`self.hp`) 0.0)
      (`GameplayStatics.SpawnEmitterAtLocation` "/Game/StarterContent/Particles/P_Explosion.P_Explosion" (`self.K2_GetActorLocation`))
      (`self.K2_DestroyActor` (`self.TargetedBybullets`))
      (`/Game/BPs/BP_wave.Remove Enemy in Array` (stale `LoadBP` wave) self)
      (`self.K2_DestroyActor`))))

(event `Refresh Text`
  (`TextRenderComponent.K2_SetText` (`self.TextRender`) (`KismetTextLibrary.Conv_StringToText` (`KismetStringLibrary.Concat_StrStr` "" (`KismetStringLibrary.Conv_DoubleToString` (`self.hp`))))))

(event `LoadBP`
  (params (wave :type "/Game/BPs/BP_wave Object Reference")))

(fn `UserConstructionScript`)