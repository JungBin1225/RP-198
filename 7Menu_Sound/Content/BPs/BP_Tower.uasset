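; Tower-defense turret that fires a BP_Bullet with a sound at enemies within range, while enabled.
; SetTower sets damage, attack delay and range, resizing the detection sphere and scaling Sphere2 to match.
; Overlap events maintain an array of BP_Enemy actors, and a Tick countdown targets the first entry whenever it expires.
; On BeginPlay it caches its location as the bullet spawn point and increments Char_KoKo's tower count.
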(event `SetTower`
  (params (Damage :type "Float (double-precision)") (Speed :type "Float (double-precision)") (Range :type "Float (double-precision)"))
  (set `self.attackdamage` Damage)
  (set `self.attackspd` Speed)
  (bind _output_get (set `self.attackrange` Range))
  (`SphereComponent.SetSphereRadius` (`self.Sphere`) _output_get true)
  (bind _returnvalue (/ _output_get 50.0))
  (`SceneComponent.SetRelativeScale3D` (`self.Sphere2`) (`KismetMathLibrary.MakeVector` _returnvalue _returnvalue 1.0)))

(event `TowerAttack`
  (params (TargetEnemy :type "/Game/BPs/BP_Enemy Object Reference"))
  (`KismetSystemLibrary.PrintString` "Tower Attacked!" false)
  (bind _returnvalue (`|SpawnActorFromClass` "/Game/BPs/BP_Bullet.BP_Bullet_C" (`KismetMathLibrary.Conv_VectorToTransform` (`self.towerlocation`)) "Undefined" "OverrideRootScale" null null))
  (`/Game/BPs/BP_Bullet.AttackToEnemy` _returnvalue (`self.attackdamage`) TargetEnemy))

(event `Enable Tower`
  ;[1 1 1] 타워 활성화/비활성화
  (set `self.Enabled` true))

(event `self.ReceiveBeginPlay`
  ;[1 1 1] Tick / 사거리 안의 적을 공격하는 조건
  (set `self.attackdelaytime` (`self.attackspd`))
  (set `self.towerlocation` (`self.K2_GetActorLocation`))
  (bind _aschar_ko_ko (cast `/Game/StarterContent/BluePrint/Char_KoKo` (`GameplayStatics.GetPlayerCharacter` 0)))
  (set `/Game/StarterContent/BluePrint/Char_KoKo.타워 수` (+ (`/Game/StarterContent/BluePrint/Char_KoKo.타워 수` _aschar_ko_ko) 1.0) _aschar_ko_ko))

(event `Disable Tower`
  ;[1 1 1] 타워 활성화/비활성화
  (set `self.Enabled` false))

(event `self.ReceiveTick`
  (params (DeltaSeconds :type "Float (single-precision)"))
  (bind _attackdelaytime (`self.attackdelaytime`))
  (bind _overlappingenemies (`self.OverlappingEnemies`))
  ;[1 1 1] Tick / 사거리 안의 적을 공격하는 조건
  (if (`self.Enabled`)
    (if (< _attackdelaytime 0.0)
      (set `self.attackdelaytime` (`self.attackspd`))
      (if (> (`KismetArrayLibrary.Array_Length` _overlappingenemies) 0)
        (`self.TowerAttack` (`|GetArrayItem` _overlappingenemies))
        (`GameplayStatics.PlaySoundAtLocation` "/Game/Sounds/TowerAttack.TowerAttack" (`self.towerlocation`) (struct) 1.0 1.0 0.0 null null null))
      (else
        (set `self.attackdelaytime` (- _attackdelaytime DeltaSeconds))))))

(event `self.ReceiveActorBeginOverlap`
  (params (OtherActor :type "Actor Object Reference"))
  ;[1 1 1] 사거리 안의 적 배열
  (bind _asbp_enemy (cast `/Game/BPs/BP_Enemy` OtherActor))
  (`KismetSystemLibrary.PrintString` "someone in radius!" false true (struct :`G` 0.66 :`B` 1.0 :`A` 1.0) 10.0)
  (`KismetArrayLibrary.Array_Add` (`self.OverlappingEnemies`) _asbp_enemy))

(event `self.ReceiveActorEndOverlap`
  (params (OtherActor :type "Actor Object Reference"))
  ;[1 1 1] 사거리 안의 적 배열
  (bind _asbp_enemy (cast `/Game/BPs/BP_Enemy` OtherActor))
  (`KismetSystemLibrary.PrintString` "someout Out of range!" false true (struct :`G` 0.66 :`B` 1.0 :`A` 1.0) 10.0)
  (`KismetArrayLibrary.Array_RemoveItem` (`self.OverlappingEnemies`) _asbp_enemy))

(fn `UserConstructionScript`)