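; Wave manager that spawns rounds of BP_Enemy at a fixed point and tracks the living ones.
; SpawnEnemy loops on a short delay, scaling HP by round and making the last enemy of every tenth round a slower, tougher boss.
; Each enemy receives a manager reference, and RemoveEnemyinArray drops it from EnemiesAlive.
; Tick resets the count and starts the next round once spawning ends and none remain alive.
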(event `self.ReceiveBeginPlay`
  (set `self.NumOfEnemy` (`self.defaultEnemyNumber`)))

(event `SpawnEnemy`
  ;[1 1 1] 적 스폰(위치 , 데이터, 개수, 라운드 조절)
  (`KismetSystemLibrary.PrintString` (`KismetStringLibrary.Concat_StrStr` "Round : " (`KismetStringLibrary.Conv_IntToString` (`self.round`))))
  (if (> (`self.NumOfEnemy`) 0) :!label _label
    (bind _returnvalue (`|SpawnActorFromClass` "/Game/BPs/BP_Enemy.BP_Enemy_C" (`KismetMathLibrary.MakeTransform` (`KismetMathLibrary.MakeVector` 11200.0 10900.0)) "Undefined" "OverrideRootScale" null null))
    ;[1 1 1] 보스 차례일때 체력계수 증가, 스피드 감소
    (if (`self.Boss`)
      (set `self.EnemyHp` 20.0)
      (set `self.EnemySpd` 0.5)
      (else
        (set `self.EnemyHp` 5.0)
        (set `self.EnemySpd` 1.0)))
    (`/Game/BPs/BP_Enemy.SetEnemyData` _returnvalue (`KismetMathLibrary.Conv_IntToDouble` (`KismetMathLibrary.FTrunc` (+ 10.0 (* (`self.EnemyHp`) (`KismetMathLibrary.Conv_IntToDouble` (`self.round`)))))) (`self.EnemySpd`))
    (set `self.NumOfEnemy` (- (`self.NumOfEnemy`) 1))
    (`KismetArrayLibrary.Array_Add` (`self.EnemiesAlive`) _returnvalue)
    (`/Game/BPs/BP_Enemy.LoadBP` _returnvalue self)
    (`KismetSystemLibrary.Delay` 0.5)
    (if (and (== (`self.NumOfEnemy`) 1) (== (`KismetMathLibrary.FMod` (`KismetMathLibrary.Conv_IntToDouble` (`self.round`)) 10.0) 0.0))
      (set `self.Boss` true)
      (`KismetSystemLibrary.PrintString` "Boss Spawned")
      (goto _label)
      (else
        (set `self.Boss` false)
        (goto _label)))
    (else
      (`KismetSystemLibrary.PrintString` (`KismetStringLibrary.Concat_StrStr` "Round" (`KismetStringLibrary.Conv_IntToString` (`self.round`)) "Spawning Ends")))))

(event `Remove Enemy in Array`
  (params (NewParam :type "/Game/BPs/BP_Enemy Object Reference"))
  (`KismetArrayLibrary.Array_RemoveItem` (`self.EnemiesAlive`) NewParam))

(event `self.ReceiveTick`
  (params (DeltaSeconds :type "Float (single-precision)"))
  ;[1 1 1] 적이 다 죽는지 확인 (라운드 타이머 추가 필요)
  (if (<= (`KismetArrayLibrary.Array_Length` (`self.EnemiesAlive`)) 0)
    (if (<= (`self.NumOfEnemy`) 0)
      (`KismetSystemLibrary.PrintString` (`KismetStringLibrary.Concat_StrStr` (`KismetStringLibrary.Conv_IntToString` (`self.round`)) "Round Completed!"))
      (set `self.NumOfEnemy` (+ (`self.defaultEnemyNumber`) 0))
      (`KismetSystemLibrary.Delay` 1.0)
      (set `self.round` (+ (`self.round`) 1))
      (`self.SpawnEnemy`))))

(fn `UserConstructionScript`)