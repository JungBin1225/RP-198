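; Wave manager that runs endless enemy rounds for what appears to be a tower defense game.
; SpawnEnemy spawns BP_Enemy at one-second intervals from a fixed point, scaling health by round and making every tenth round's last enemy a slower boss.
; Tick watches the EnemiesAlive array and starts a larger round after a delay once cleared.
; Each wave drains Char_KoKo's power per tower, overwriting Hp with the difference when power is insufficient.
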(event `SpawnEnemy`
  ;[1 1 1] 적 스폰(위치 , 데이터, 개수, 라운드 조절)
  (`self.전력 소모`)
  (`KismetSystemLibrary.PrintString` (`KismetStringLibrary.Concat_StrStr` "Round : " (`KismetStringLibrary.Conv_IntToString` (`self.round`))))
  (if (> (`self.NumOfEnemy`) 0) :!label _label
    (bind _returnvalue (`|SpawnActorFromClass` "/Game/BPs/BP_Enemy.BP_Enemy_C" (`KismetMathLibrary.MakeTransform` (`KismetMathLibrary.MakeVector` 11200.0 10900.0)) "Undefined" "OverrideRootScale" null null))
    ;[1 1 1] 보스 차례일때 체력계수 증가, 스피드 감소
    (if (`self.Boss`)
      (set `self.EnemyHp` 200.0)
      (set `self.EnemySpd` 2.0)
      (else
        (set `self.EnemyHp` 10.0)
        (set `self.EnemySpd` 4.0)))
    (`/Game/BPs/BP_Enemy.SetEnemyData` _returnvalue (`KismetMathLibrary.Conv_IntToDouble` (`KismetMathLibrary.FTrunc` (+ 10.0 (* (`self.EnemyHp`) (`KismetMathLibrary.Conv_IntToDouble` (`self.round`)))))) (`self.EnemySpd`))
    (set `self.NumOfEnemy` (- (`self.NumOfEnemy`) 1))
    (`KismetArrayLibrary.Array_Add` (`self.EnemiesAlive`) _returnvalue)
    (`/Game/BPs/BP_Enemy.LoadBP` _returnvalue self)
    (`KismetSystemLibrary.Delay` 1.0)
    (if (and (== (`self.NumOfEnemy`) 1) (== (`KismetMathLibrary.FMod` (`KismetMathLibrary.Conv_IntToDouble` (`self.round`)) 10.0) 0.0))
      (set `self.Boss` true)
      (`KismetSystemLibrary.PrintString` "Boss Spawned" false)
      (goto _label)
      (else
        (set `self.Boss` false)
        (goto _label)))
    (else
      (`KismetSystemLibrary.PrintString` (`KismetStringLibrary.Concat_StrStr` "Round" (`KismetStringLibrary.Conv_IntToString` (`self.round`)) "Spawning Ends")))))

(event `self.ReceiveBeginPlay`
  (set `self.NumOfEnemy` (`self.defaultEnemyNumber`))
  (`KismetSystemLibrary.Delay` 10.0)
  (`self.SpawnEnemy`))

(event `Remove Enemy in Array`
  (params (NewParam :type "/Game/BPs/BP_Enemy Object Reference"))
  (`KismetArrayLibrary.Array_RemoveItem` (`self.EnemiesAlive`) NewParam))

(event `self.ReceiveTick`
  (params (DeltaSeconds :type "Float (single-precision)"))
  ;[1 1 1] 적이 다 죽는지 확인 (라운드 타이머 추가 필요)
  (if (<= (`KismetArrayLibrary.Array_Length` (`self.EnemiesAlive`)) 0)
    (if (<= (`self.NumOfEnemy`) 0)
      (`KismetSystemLibrary.PrintString` (`KismetStringLibrary.Concat_StrStr` (`KismetStringLibrary.Conv_IntToString` (`self.round`)) "Round Completed!"))
      (set `self.NumOfEnemy` (+ (`self.defaultEnemyNumber`) (`self.round`)))
      (`KismetSystemLibrary.Delay` 10.0)
      (set `self.round` (+ (`self.round`) 1))
      (`self.SpawnEnemy`))))

(event `전력 소모`
  ;[1 1 1] 웨이브 시작 시 전력 소모
  (bind _aschar_ko_ko (cast `/Game/StarterContent/BluePrint/Char_KoKo` (`GameplayStatics.GetPlayerCharacter` 0)))
  (bind `_전력` (`/Game/StarterContent/BluePrint/Char_KoKo.전력` _aschar_ko_ko))
  (bind _returnvalue (* (`/Game/StarterContent/BluePrint/Char_KoKo.타워 수` _aschar_ko_ko) 1.0))
  (if (> `_전력` _returnvalue)
    (bind _returnvalue_2 (- `_전력` _returnvalue))
    (set `/Game/StarterContent/BluePrint/Char_KoKo.전력` _returnvalue_2 _aschar_ko_ko)
    (else
      (set `/Game/StarterContent/BluePrint/Char_KoKo.Hp` _returnvalue_2 _aschar_ko_ko))))

(fn `UserConstructionScript`)