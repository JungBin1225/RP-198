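; BP_Bullet is a homing projectile that chases an assigned enemy and damages it on contact.
; AttackToEnemy stores the target and registers the bullet with it through TargetedBybullet.
; Tick applies a fixed per-frame local offset, unscaled by delta time, along the direction to the enemy's Enemylocation.
; When Tick detects overlap with the target, it calls GetAttacked with the damage and destroys itself.
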(event `self.ReceiveTick`
  (params (DeltaSeconds :type "Float (single-precision)"))
  (bind _targetenemy (`self.TargetEnemy`))
  (`self.K2_AddActorLocalOffset` (* (`KismetMathLibrary.GetDirectionUnitVector` (`self.K2_GetActorLocation`) (`/Game/BPs/BP_Enemy.Enemylocation` _targetenemy)) 50.0))
  (if (`self.IsOverlappingActor` _targetenemy)
    (`/Game/BPs/BP_Enemy.GetAttacked` (stale `AttackToEnemy` _output_get) (stale `AttackToEnemy` damage) self)
    (`self.K2_DestroyActor`)))

(event `AttackToEnemy`
  (params (damage :type "Float (double-precision)") (target :type "/Game/BPs/BP_Enemy Object Reference"))
  (bind _output_get (set `self.TargetEnemy` target))
  (`/Game/BPs/BP_Enemy.targetedBybullet` target self))

(event `self.ReceiveBeginPlay`)

(fn `UserConstructionScript`)