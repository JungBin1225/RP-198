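; BP_Crafting_table is a crafting table actor that signals the main UI when the player is in range.
; Overlap events on its Sphere component set a Visible flag for the player character and copy it to the first top-level MainUI widget found, apparently to toggle popup text.
; BeginPlay enables input from the first player controller for clicking, though the file contains no click handling or crafting logic.
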(event `self.Sphere.OnComponentBeginOverlap`
  (params (OverlappedComponent :type "PrimitiveComponent Object Reference") (OtherActor :type "Actor Object Reference") (OtherComp :type "PrimitiveComponent Object Reference") (OtherBodyIndex :type Integer) (bFromSweep :type Boolean) (SweepResult :type "HitResult Structure (by ref)"))
  ;[1 1 1] 팝업 텍스트 설정
  (if (== OtherActor (`GameplayStatics.GetPlayerCharacter` 0))
    (bind _output_get (set `self.visible` true))
    (bind _foundwidgets (`WidgetBlueprintLibrary.GetAllWidgetsOfClass` "/Game/BPs/MainUI.MainUI_C"))
    (set `/Game/BPs/MainUI.visible` _output_get (`|GetArrayItem` _foundwidgets))))

(event `self.Sphere.OnComponentEndOverlap`
  (params (OverlappedComponent :type "PrimitiveComponent Object Reference") (OtherActor :type "Actor Object Reference") (OtherComp :type "PrimitiveComponent Object Reference") (OtherBodyIndex :type Integer))
  ;[1 1 1] 팝업 텍스트 설정
  (if (== OtherActor (`GameplayStatics.GetPlayerCharacter` 0))
    (bind _output_get (set `self.visible` false))
    (bind _foundwidgets (`WidgetBlueprintLibrary.GetAllWidgetsOfClass` "/Game/BPs/MainUI.MainUI_C"))
    (set `/Game/BPs/MainUI.visible` _output_get (`|GetArrayItem` _foundwidgets))))

(event `self.ReceiveBeginPlay`
  ;[1 1 1] 클릭 가능하게 하기
  (`self.EnableInput` (`GameplayStatics.GetPlayerController` 0)))

(fn `UserConstructionScript`)