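; BP_wave is a round-based wave spawner that sends escalating groups of BP_Enemy.
; SpawnEnemy uses a delayed loop to spawn enemies at a randomized X position, scale health by round, register them in EnemiesAlive and pass itself to each.
; RemoveEnemyinArray drops enemies from that array.
; Tick detects a cleared wave, refills the round-scaled count before a pause, then advances the round and restarts spawning.
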(event `SpawnEnemy`
  (`KismetSystemLibrary.PrintString` (`KismetStringLibrary.Concat_StrStr` "Round : " (`KismetStringLibrary.Conv_IntToString` (`self.round`))))
  (if (> (`self.NumOfEnemy`) 0) :!label _label
    (bind _returnvalue (`|SpawnActorFromClass` "/Game/BPs/BP_Enemy.BP_Enemy_C" (`KismetMathLibrary.MakeTransform` (`KismetMathLibrary.MakeVector` (+ (- (* (`KismetMathLibrary.RandomFloat`) 1000.0) 500.0) 10000.0) 11000.0)) "Undefined" "OverrideRootScale" null null))
    (`/Game/BPs/BP_Enemy.SetEnemyData` _returnvalue (`KismetMathLibrary.Conv_IntToDouble` (`KismetMathLibrary.FTrunc` (+ 10.0 (* 5.0 (`KismetMathLibrary.Conv_IntToDouble` (`self.round`)))))) 2.0)
    (set `self.NumOfEnemy` (- (`self.NumOfEnemy`) 1))
    (`KismetArrayLibrary.Array_Add` (`self.EnemiesAlive`) _returnvalue)
    (`/Game/BPs/BP_Enemy.LoadBP` _returnvalue self)
    (`KismetSystemLibrary.Delay` 0.5)
    (goto _label)
    (else
      (`KismetSystemLibrary.PrintString` (`KismetStringLibrary.Concat_StrStr` "Round" (`KismetStringLibrary.Conv_IntToString` (`self.round`)) "Spawning Ends")))))

(event `Remove Enemy in Array`
  (params (NewParam :type "/Game/BPs/BP_Enemy Object Reference"))
  (`KismetArrayLibrary.Array_RemoveItem` (`self.EnemiesAlive`) NewParam))

(event `self.ReceiveTick`
  (params (DeltaSeconds :type "Float (single-precision)"))
  (if (<= (`KismetArrayLibrary.Array_Length` (`self.EnemiesAlive`)) 0)
    (if (<= (`self.NumOfEnemy`) 0)
      (`KismetSystemLibrary.PrintString` (`KismetStringLibrary.Concat_StrStr` (`KismetStringLibrary.Conv_IntToString` (`self.round`)) "Round Completed!"))
      (set `self.NumOfEnemy` (+ 10 (`self.round`)))
      (`KismetSystemLibrary.Delay` 3.0)
      (set `self.round` (+ (`self.round`) 1))
      (`self.SpawnEnemy`))))

(fn `UserConstructionScript`)